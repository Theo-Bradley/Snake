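; MyHUD is a Blueprint that owns the game's on-screen UI and relays score and restart events to it.
; On BeginPlay it creates the UI_widget, stores the reference and adds it to the viewport.
; UpdateScore copies its Score variable into the widget and triggers the widget's update, while ShowRestart calls the widget's restart display event.
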(event Custom|Event%20ShowRestart
  (Default|EventShowRestart (Variables|Default|GetUIWidget)))

(event Custom|Event%20UpdateScore
  (bind _uiwidget (Variables|Default|GetUIWidget))
  (Variables|/Game/Blueprints/UI_widget.UI_widget_C|SetScore _uiwidget (Variables|Default|GetScore))
  (Default|UpdateScore _uiwidget))

(event EventBeginPlay
  (bind _returnvalue (UserInterface|CreateWidget "/Game/Blueprints/UI_widget.UI_widget_C"))
  (bind _output_get (Variables|Default|SetUIWidget _returnvalue))
  (UserInterface|Viewport|AddtoViewport _output_get 0))

(event Collision|EventActorBeginOverlap
  (params (OtherActor :type Actor%20Object%20Reference)))

(event EventTick
  (params (DeltaSeconds :type Float%20%28single-precision%29)))

(fn ConstructionScript)