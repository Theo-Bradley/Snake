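; PrimaryPart is the head of a Snake-style game, spawning a top-down camera and turning with directional input, blocking reversals against the last step's rotation.
; Tick moves it forward at timed steps and passes its old position to a linked chain of SecondaryParts.
; Overlapping a FoodPill adds score, relocates the pill randomly and appends a part to the tail.
; Overlapping another Part calls Die, which only prints a placeholder string.
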(event OnComponentBeginOverlap(Mesh)
  (params (OverlappedComponent :type Primitive%20Component%20Object%20Reference) (OtherActor :type Actor%20Object%20Reference) (OtherComp :type Primitive%20Component%20Object%20Reference) (OtherBodyIndex :type Integer) (bFromSweep :type Boolean) (SweepResult :type Hit%20Result%20Structure%20%28by%20ref%29))
  (bind _returnvalue (Utilities|GetObjectName OtherActor))
  (bind _spawnbounds (Variables|Default|GetspawnBounds))
  (bind (_x _y) (Math|Vector2D|BreakVector2D _spawnbounds))
  (if (Utilities|String|Contains _returnvalue "FoodPill")
    (Variables|Default|SetScore (+ 1 (Variables|Default|GetScore)))
    (Transformation|SetActorLocation OtherActor (Math|Vector|MakeVector (- (* (Math|Random|RandomFloat) (* 2.0 _x)) _x) (- (* (* _y 2.0) (Math|Random|RandomFloat)) _y) 8e+01) false false)
    ;[1 1 1] Get end part (no ChildPart)
    (if (Utilities|IsValid (Variables|Default|GetChildPart))
      (Variables|Default|SetcurrentChildPart (Variables|Default|GetChildPart))
      (while (Utilities|IsValid (Variables|/Game/Blueprints/SecondaryPart.SecondaryPart_C|GetChildPart (Variables|Default|GetcurrentChildPart)))
        (Variables|Default|SetcurrentChildPart (Variables|/Game/Blueprints/SecondaryPart.SecondaryPart_C|GetChildPart (Variables|Default|GetcurrentChildPart))))
      (bind _returnvalue_2 (Game|SpawnActorfromClass "/Game/Blueprints/SecondaryPart.SecondaryPart_C" (Math|Transform|MakeTransform (+ (Transformation|GetActorLocation (Variables|Default|GetcurrentChildPart)) (* (Transformation|GetActorForwardVector (Variables|Default|GetcurrentChildPart)) "-125.000000,0.000000,0.000000"))) "AlwaysSpawn" "MultiplyWithRoot" 0 0))
      (Variables|/Game/Blueprints/SecondaryPart.SecondaryPart_C|SetChildPart (Variables|Default|GetcurrentChildPart) _returnvalue_2)
      (else
        (bind _returnvalue_3 (Game|SpawnActorfromClass "/Game/Blueprints/SecondaryPart.SecondaryPart_C" (Math|Transform|MakeTransform (+ (Transformation|GetActorLocation) (* (Transformation|GetActorForwardVector) "-125.000000,0.000000,0.000000"))) "AlwaysSpawn" "MultiplyWithRoot" 0 0))
        (Variables|Default|SetChildPart _returnvalue_3)))
    (elif (Utilities|String|Contains _returnvalue "Part")
      (CallFunction|Die))))

(event EventBeginPlay
  (bind _returnvalue (Game|SpawnActorfromClass "/Script/Engine.CameraActor" (Math|Transform|MakeTransform "0.000000,0.000000,1500.000000" "-90.000000,0.000000,0.000000") "Undefined" "MultiplyWithRoot" 0 0))
  (Variables|Default|SetbFindCameraComponentWhenViewTarget true)
  (Game|Player|SetViewTargetwithBlend (Game|GetPlayerController 0) _returnvalue 0.0 "VTBlend_Linear" 0.0 false))

(event Collision|EventActorBeginOverlap
  (params (OtherActor :type Actor%20Object%20Reference)))

(event EventTick
  (params (DeltaSeconds :type Float%20%28single-precision%29))
  (bind _childpart (Variables|Default|GetChildPart))
  (Variables|Default|SetoldPos (Transformation|GetActorLocation))
  ;[1 1 1] Move Along local forward
  (if (>= (Utilities|Time|GetTimeSeconds) (Variables|Default|GetnextMoveStep))
    (Variables|Default|SetcurrentRot (Transformation|GetActorRotation))
    (Transformation|SetActorLocation (+ (Transformation|GetActorLocation) (* (Transformation|GetActorForwardVector) (Variables|Default|GetMoveAmt))) false false)
    (Variables|Default|SetnextMoveStep (+ (Variables|Default|GetnextMoveStep) (Variables|Default|GetStepSpeed)))
    (if (Utilities|IsValid (Variables|Default|GetChildPart))
      (Variables|/Game/Blueprints/SecondaryPart.SecondaryPart_C|SetNextPos _childpart (Variables|Default|GetoldPos))
      (Default|MoveEvent _childpart))))

(event Input|ActionEvents|InputActionLeft
  (params (Key :type Key%20Structure :default "None"))
  (:Pressed
    (if (!= (.Yaw (Math|Rotator|BreakRotator (Variables|Default|GetcurrentRot))) 9e+01)
      (Transformation|SetActorRotation "0.000000,-90.000000,0.000000"))))

(event Input|ActionEvents|InputActionRight
  (params (Key :type Key%20Structure :default "None"))
  (:Pressed
    (if (!= (.Yaw (Math|Rotator|BreakRotator (Variables|Default|GetcurrentRot))) -9e+01)
      (Transformation|SetActorRotation "0.000000,90.000000,0.000000"))))

(event Input|ActionEvents|InputActionUp
  (params (Key :type Key%20Structure :default "None"))
  (:Pressed
    (if (!= (.Yaw (Math|Rotator|BreakRotator (Variables|Default|GetcurrentRot))) 1.8e+02)
      (Transformation|SetActorRotation "0, 0, 0"))))

(event Input|ActionEvents|InputActionDown
  (params (Key :type Key%20Structure :default "None"))
  (:Pressed
    (if (!= (.Yaw (Math|Rotator|BreakRotator (Variables|Default|GetcurrentRot))) 0.0)
      (Transformation|SetActorRotation "0.000000,180.000000,0.000000"))))

(fn ConstructionScript)

(fn Die
  (Development|PrintString "Hello"))